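; Player inventory component that stores ammo counts and quest items in name-keyed maps and routes item pickups by type.
; Weapon and melee pickups go out through CallPickUpWeapon and CallPickUpWeaponMelee, while ammo and quest items add to their map counts.
; Ammo must already exist as a map key; its pickup sends a HUD message, and unknown types print an error.
; Quest items can be queried and removed, dropping the entry at zero.
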(event `self.ReceiveBeginPlay`
  (bind _output_get (set `self.PlayerCharacter` (`self.GetOwner`)))
  (set `self.PlayerWeaponStorage` (`Actor.GetComponentByClass` _output_get "/Game/Interaction/Blueprints/Pawn/Player/Components/BP_WeaponStorage.BP_WeaponStorage_C")))

(event `PickUpItem`
  (params (Name :type String) (ItemType :type "/Game/Interaction/Blueprints/Pawn/Player/Components/Enum_ItemType Enum" :default "NewEnumerator0") (NumberOfItems :type Integer) (ItemImage :type "Texture2D Object Reference") (TakeWeaponInHands :type Boolean) (CustomWeapon :type Boolean) (WeaponParam :type "/Game/Interaction/Blueprints/Weapon/Structures/Struct_W Structure"))
  (switch `/Game/Interaction/Blueprints/Pawn/Player/Components/Enum_ItemType` ItemType
    (:`NewEnumerator0`
      (`self.PickUpWeapon` Name TakeWeaponInHands CustomWeapon WeaponParam))
    (:`NewEnumerator3`
      (`self.PickUpWeaponMelee` Name))
    (:`NewEnumerator1`
      (`self.AddAmmo` Name NumberOfItems ItemImage))
    (:`NewEnumerator2`
      (`self.AddQuestItem` Name NumberOfItems))))

(event `RemoveAllItems`
  (`BlueprintMapLibrary.Map_Clear` (`self.AmmoType`))
  (`BlueprintMapLibrary.Map_Clear` (`self.QuestItems`)))

(fn `AddAmmo`
  (params (AmmoType :type String) (NumberOfAmmo :type Integer) (AmmoImage :type "Texture2D Object Reference"))
  (bind (_value _returnvalue) (`BlueprintMapLibrary.Map_Find` (`self.AmmoType`) AmmoType))
  (if _returnvalue
    (bind _hud (message `/Game/Interaction/Blueprints/Pawn/Player/StatusInterface.GetComponents` (`self.GetOwner`)))
    (message `/Game/Interaction/Hud/BI_Hud.Hud_PickUpAmmo` _hud AmmoType _value NumberOfAmmo AmmoImage)
    (`BlueprintMapLibrary.Map_Add` (`self.AmmoType`) AmmoType (+ _value NumberOfAmmo))
    (else
      (`KismetSystemLibrary.PrintString` "Type ammo does not exist. Check the list of \"AmmoType\" in the inventory (Map Varible)"))))

(fn `AddQuestItem`
  (params (ItemName :type String) (NumberOfItems :type Integer :default 1))
  (bind _questitems (`self.QuestItems`))
  (bind (_value _returnvalue) (`BlueprintMapLibrary.Map_Find` (`self.QuestItems`) ItemName))
  (if _returnvalue
    (`BlueprintMapLibrary.Map_Add` _questitems ItemName (+ _value NumberOfItems))
    (else
      (`BlueprintMapLibrary.Map_Add` _questitems ItemName NumberOfItems))))

(fn `GetAmmo`
  (params (AmmoName :type "String (by ref)"))
  (returns (AmmoCount :type Integer))
  (return (`BlueprintMapLibrary.Map_Find` (`self.AmmoType`) AmmoName)))

(fn `GetQuestItem`
  (params (Key :type String))
  (returns (ItemInInventory :type Boolean) (NumberOfItems :type Integer))
  (bind (_value _returnvalue) (`BlueprintMapLibrary.Map_Find` (`self.QuestItems`) Key))
  (return _returnvalue _value))

(fn `RemoveQuestItem`
  (params (ItemName :type String) (NumberOfItems :type Integer :default 1))
  (bind (_value _returnvalue) (`BlueprintMapLibrary.Map_Find` (`self.QuestItems`) ItemName))
  (bind _returnvalue_2 (- _value NumberOfItems))
  (if _returnvalue
    (if (> _returnvalue_2 0)
      (`BlueprintMapLibrary.Map_Add` (`self.QuestItems`) ItemName _returnvalue_2)
      (else
        (`BlueprintMapLibrary.Map_Remove` (`self.QuestItems`) ItemName)))))